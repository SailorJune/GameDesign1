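; Finish-line lap timer that reports lap times for the custom third-person character through debug Print String messages.
; From BeginPlay, OnscreenTimer re-calls itself after a short Delay, printing the real time elapsed since LastTimeStamp.
; When BP_ThirdPersonCharacterCustom begins overlapping the Box, it prints the lap time and resets LastTimeStamp.
; BeginPlay leaves LastTimeStamp untouched, so the first lap counts from that variable's default value.
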(event `Onscreen Timer`
  (`KismetSystemLibrary.PrintString` (`KismetStringLibrary.Concat_StrStr` "Current Lap: " (`KismetTextLibrary.Conv_TextToString` (`KismetTextLibrary.Conv_DoubleToText` (- (`GameplayStatics.GetRealTimeSeconds`) (`self.LastTimeStamp`)) "HalfToEven" false true 1 324 0 1)) " Seconds ") true true (struct :`G` 0.66 :`B` 1.0 :`A` 1.0) 0.1)
  (`KismetSystemLibrary.Delay` 0.1)
  (`self.Onscreen Timer`))

(event `self.ReceiveBeginPlay`
  (`self.Onscreen Timer`))

(event `self.Box.OnComponentBeginOverlap`
  (params (OverlappedComponent :type "PrimitiveComponent Object Reference") (OtherActor :type "Actor Object Reference") (OtherComp :type "PrimitiveComponent Object Reference") (OtherBodyIndex :type Integer) (bFromSweep :type Boolean) (SweepResult :type "HitResult Structure (by ref)"))
  (cast `/Game/Blueprints/BP_ThirdPersonCharacterCustom` OtherActor)
  (`KismetSystemLibrary.PrintString` (`KismetStringLibrary.Concat_StrStr` "That lap took " (`KismetTextLibrary.Conv_TextToString` (`KismetTextLibrary.Conv_DoubleToText` (- (`GameplayStatics.GetRealTimeSeconds`) (`self.LastTimeStamp`)) "HalfToEven" false true 1 324 0 1)) " Seconds!"))
  (set `self.LastTimeStamp` (`GameplayStatics.GetRealTimeSeconds`)))

(fn `UserConstructionScript`)