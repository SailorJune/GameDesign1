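; Interactable turn station whose Inside component rotates on its yaw axis, up to a 90-degree scale, once powered.
; A capsule overlap with the custom third-person character toggles the interact widget and tracks whether the player is in range.
; The Turn event flip-flops an interacting flag, replaying the rotation timeline from the start when that flag, overlap and power are all true.
; A separate Powered event enables power.
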(event `self.ReceiveBeginPlay`
  (bind _returnvalue (`|CreateWidget` "/Game/Widgets/W_interact.W_interact_C"))
  (set `self.InteractWidget` _returnvalue))

(event `Turn`
  (bind _isa (`/Engine/EditorBlueprintResources/StandardMacros.FlipFlop`)
    (:`A`
      (set `self.Interacting` _isa))
    (:`B`
      (set `self.Interacting` false)))
  (if (and (`self.Interacting`) (stale `self.Capsule.OnComponentBeginOverlap` _output_get) (`self.Power`))
    (`KismetSystemLibrary.PrintString` "ROTATION")
    (bind (_direction _rotate) (`Timeline|Rotate Inside` :!via `PlayFromStart`)
      (:`Update`
        (`SceneComponent.K2_SetRelativeRotation` (`self.Inside`) (`KismetMathLibrary.MakeRotator` 0.0 0.0 (* _rotate 90.0)) false false)))))

(event `Powered`
  (set `self.Power` true))

(event `self.Capsule.OnComponentBeginOverlap`
  (params (OverlappedComponent :type "PrimitiveComponent Object Reference") (OtherActor :type "Actor Object Reference") (OtherComp :type "PrimitiveComponent Object Reference") (OtherBodyIndex :type Integer) (bFromSweep :type Boolean) (SweepResult :type "HitResult Structure (by ref)"))
  (cast `/Game/Blueprints/BP_ThirdPersonCharacterCustom` OtherActor)
  (`UserWidget.AddToViewport` (`self.InteractWidget`) 0)
  (bind _output_get (set `self.Overlaping` true)))

(event `self.Capsule.OnComponentEndOverlap`
  (params (OverlappedComponent :type "PrimitiveComponent Object Reference") (OtherActor :type "Actor Object Reference") (OtherComp :type "PrimitiveComponent Object Reference") (OtherBodyIndex :type Integer))
  (cast `/Game/Blueprints/BP_ThirdPersonCharacterCustom` OtherActor)
  (`Widget.RemoveFromParent` (`self.InteractWidget`))
  (set `self.Overlaping` false))

(fn `UserConstructionScript`)